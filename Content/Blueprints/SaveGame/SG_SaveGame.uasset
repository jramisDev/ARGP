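; SG_SaveGame is a save game Blueprint that stores a character's skill state.
; SavePlayerData copies SkillsIDs and AllAvailableSkills from the BaseCharacter's BPCSkillManager component into its own variables and returns itself.
; LoadData writes both stored values straight back into that component, with no disk save or load in either function.
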(fn SavePlayerData
  (params (Base%20Character :type BP%20Base%20Character%20Object%20Reference))
  (bind _bpc_skillmanager (Variables|/Game/Blueprints/Characters/BP_BaseCharacter.BP_BaseCharacter_C|GetBPC_SkillManager Base%20Character))
  (Variables|Default|SetSkillsIDs (Variables|/Game/Blueprints/Components/BPC_SkillManager.BPC_SkillManager_C|GetSkillsIDs _bpc_skillmanager))
  (Variables|Default|SetAllAvailableSkills (Variables|/Game/Blueprints/Components/BPC_SkillManager.BPC_SkillManager_C|GetAllAvailableSkills _bpc_skillmanager))
  (return self))

(fn LoadData
  (params (Base%20Character :type BP%20Base%20Character%20Object%20Reference))
  (bind _bpc_skillmanager (Variables|/Game/Blueprints/Characters/BP_BaseCharacter.BP_BaseCharacter_C|GetBPC_SkillManager Base%20Character))
  (Variables|/Game/Blueprints/Components/BPC_SkillManager.BPC_SkillManager_C|SetSkillsIDs _bpc_skillmanager (Variables|Default|GetSkillsIDs))
  (Variables|/Game/Blueprints/Components/BPC_SkillManager.BPC_SkillManager_C|SetAllAvailableSkills _bpc_skillmanager (Variables|Default|GetAllAvailableSkills)))