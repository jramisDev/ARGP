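; Quest objective Blueprint that tracks progress toward a kill-count goal within a quest.
; Construct stores the objective data struct and its ID.
; AddOneKillToCount increments the count when the objective is of the first enum type and the killed class matches its target actor.
; It prints progress on screen, or a completion message once the quantity is reached, then calls ObjectiveCompleted with the quest and objective IDs.
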(fn Construct
  (params (QuestObjetive :type S%20Quest%20Objective%20Structure%20%28by%20ref%29) (ID%20Requisite :type Integer%20%28by%20ref%29))
  (Variables|Default|SetQuest%20Objetive QuestObjetive)
  (Variables|Default|SetIdObjective ID%20Requisite))

(fn AddOneKilltoCount
  (params (Enemy%20Class :type BP%20Base%20Enemy%20Soft%20Class%20Reference%20%28by%20ref%29))
  (bind _quest_objetive (Variables|Default|GetQuest%20Objetive))
  (bind (_type _quantity _actor) (Utilities|Struct|BreakS_QuestObjective _quest_objetive))
  (if (Utilities|Enum|Equal(Enum) _type "NewEnumerator0")
    (if (== Enemy%20Class _actor)
      (bind _result (Math|Integer|IncrementInt (Variables|Default|GetCurrentQuantity))
        (:%20%20
          (if (<= _quantity _result)
            (Development|PrintString 0 "Objective Completed" true true "(R=0.962303,G=1.000000,B=0.000000,A=1.000000)")
            (Default|CallObjectiveCompleted (Variables|Default|GetIDQuest) (Variables|Default|GetIdObjective))
            (else
              (Development|PrintText 0 (Utilities|Text|FormatText "{a} / {b}" (Variables|Default|GetCurrentQuantity) _quantity)))))))))