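; BP_P_SuperNova is a skill actor, a child Blueprint that spawns a follow-up skill when it starts to die.
; PreInit assigns Sphere1 as its damage collision.
; StartDie looks up the SpawnAditionalClass row in DT_Skills and spawns that skill's class at its own transform, passing along the row data, owner and instigator.
; The parent death logic then runs, even if no row is found.
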(event EventBeginPlay
  (|CallParentFunction) ; This node is disabled and will not be called.\nDrag off pins to build functionality.
)

(event EventStartDie
  (bind _returnvalue (Utilities|GetDataTableRow "/Game/Blueprints/DataTables/DT_Skills.DT_Skills" (.SpawnAditionalClass (Utilities|Struct|BreakS_Skills (Variables|Default|GetSkillData))))
    (:then
      (Game|SpawnActorfromClass (.SkillBase (Utilities|Struct|BreakS_Skills _returnvalue)) (Math|Transform|MakeTransform (Transformation|GetActorLocation) (Transformation|GetActorRotation) "1.000000,1.000000,1.000000") "Undefined" "MultiplyWithRoot" (Components|GetOwner) _returnvalue (Game|GetInstigator))
      (|CallParentFunction))
    (:RowNotFound
      (|CallParentFunction))))

(fn ConstructionScript
  (|CallParentFunction))

(fn PreInit
  (Variables|Default|SetCollisionDamage (Variables|Default|GetSphere1)))