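; BP_Launch is a child skill Blueprint that launches a damaged BP_BaseCharacter vertically.
; PreInit assigns the Capsule as the damage collision used by the parent skill logic.
; StartDie applies the launch and calls the parent's death handling only if the instigator is not jumping.
; If the cast fails or the instigator is jumping, neither the launch nor the parent StartDie runs.
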(event EventStartDie
  (bind _asbp_base_character (Utilities|Casting|CastToBP_BaseCharacter (Variables|Default|GetDamaged%20Actor)))
  (if (not (Variables|/Game/Blueprints/Characters/BP_BaseCharacter.BP_BaseCharacter_C|GetIsJumping (CallFunction|GetInstigatorRef)))
    (Character|LaunchCharacter _asbp_base_character (Math|Vector|MakeVector 0.0 0.0 (Variables|Default|GetLaunch%20Velocity%20Z)) false false)
    (|CallParentFunction)))

(fn ConstructionScript
  (|CallParentFunction))

(fn PreInit
  (Variables|Default|SetCollisionDamage (Variables|Default|GetCapsule)))