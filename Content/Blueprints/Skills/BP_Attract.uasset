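; BP_Attract is a skill actor that pulls a character in front of it back toward itself when spawned.
; On BeginPlay it line traces forward up to AttrackDistance on the Pawn profile, with debug drawing on.
; A hit BP_BaseCharacter receives a velocity-change impulse opposite the actor's forward vector.
; The impulse strength is interpolated by hit distance, so farther targets are pulled harder.
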(event EventBeginPlay
  (bind _returnvalue (Transformation|GetActorLocation))
  (bind (_outhit _returnvalue_2) (Class|KismetSystemLibrary|LineTraceSinglebyProfile _returnvalue (+ _returnvalue (* (Transformation|GetActorForwardVector) (Variables|Default|GetAttrackDistance))) "Pawn" false 0 "ForDuration" true))
  (if _returnvalue_2
    (bind _asbp_base_character (Utilities|Casting|CastToBP_BaseCharacter (.HitActor (Collision|BreakHitResult _outhit))))
    (Physics|AddImpulse (Variables|/Script/Engine.Character|GetCharacterMovement _asbp_base_character) (* (Transformation|GetActorForwardVector) (* (Math|Float|Lerp 1e+03 1.5e+04 (/ (Math|Vector|Distance(Vector) (Transformation|GetActorLocation) (.ImpactPoint (Collision|BreakHitResult _outhit))) (Variables|Default|GetAttrackDistance))) -1.0)) true)))

(fn ConstructionScript
  (|CallParentFunction))