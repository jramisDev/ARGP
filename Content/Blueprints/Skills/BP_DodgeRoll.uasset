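; BP_DodgeRoll is a skill Blueprint that performs a dodge roll on its instigator.
; On BeginPlay, only if the instigator is not jumping, it clears IsDodgin, plays the SkillData montage on the instigator, then runs the parent BeginPlay.
; A jumping instigator skips all of this, including the parent call.
; StartDie also clears IsDodgin; nothing here sets that flag to true.
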(event EventBeginPlay
  (bind _as_bp_base_character (CallFunction|GetInstigatorRef))
  (if (not (Variables|/Game/Blueprints/Characters/BP_BaseCharacter.BP_BaseCharacter_C|GetIsJumping (CallFunction|GetInstigatorRef)))
    (Variables|/Game/Blueprints/Characters/BP_BaseCharacter.BP_BaseCharacter_C|SetIsDodgin _as_bp_base_character false)
    (Animation|PlayAnimMontage _as_bp_base_character (.AnimMontage (Utilities|Struct|BreakS_Skills (Variables|Default|GetSkillData))) 1.0 "None")
    (|CallParentFunction)))

(event EventStartDie
  (Variables|/Game/Blueprints/Characters/BP_BaseCharacter.BP_BaseCharacter_C|SetIsDodgin (CallFunction|GetInstigatorRef) false))

(fn ConstructionScript
  (|CallParentFunction))