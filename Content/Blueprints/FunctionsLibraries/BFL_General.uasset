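; BFL_General is a general function library with SortArrayInteger, which returns an integer array in ascending order.
; It works as a selection sort: it repeatedly finds the minimum in a local copy, appends it to the result and removes it from the copy.
; The append uses AddUnique, so duplicate values appear only once in the result.
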(fn SortArrayInteger
  (params (Array :type Array%20of%20Integers))
  (LocalVariables|SetNewLocalVar Array)
  (while (Utilities|Array|IsNotEmpty (LocalVariables|GetNewLocalVar))
    (Utilities|Array|AddUnique (LocalVariables|GetBueno) (.MinValue (Math|Integer|MinOfIntArray (LocalVariables|GetNewLocalVar))))
    (Utilities|Array|RemoveIndex (LocalVariables|GetNewLocalVar) (.IndexOfMinValue (Math|Integer|MinOfIntArray (LocalVariables|GetNewLocalVar)))))
  (return (LocalVariables|GetBueno)))