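; Quest manager component that loads every quest from DT_Quest at BeginPlay and is meant to track kill objectives.
; AddNewQuest stores each row by ID, creates a QuestProgressItem in KillingQuests and rebuilds the Enemys list from objective actors.
; EnemyKilled finds entries whose Enemies contain the victim and calls UpdateQuestProgress with their keys.
; Progress tracking is unfinished: UpdateQuestProgress only loops over objectives with an empty body.
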(event EventBeginPlay
  (bind _outrownames (DataTable|GetDataTableRowNames "/Game/Blueprints/DataTables/DT_Quest.DT_Quest"))
  (for _array_element _outrownames
    (CallFunction|AddNewQuest _array_element)))

(fn EnemyKilled
  (params (Enemy :type BP%20Base%20Enemy%20Soft%20Class%20Reference))
  (bind _values (Utilities|Map|Values 0))
  (for (_array_element _array_index) _values
    (if (Utilities|Array|ContainsItem (Utilities|Struct|BreakS_EnemyArray _array_element) Enemy)
      (bind _keys (Utilities|Map|Keys 0))
      (CallFunction|UpdateQuestProgress (Utilities|Array|Get(acopy) _keys _array_index) "None"))))

(fn AddNewQuest
  (params (ID%20Quest :type Name))
  (bind _returnvalue (Utilities|GetDataTableRow "/Game/Blueprints/DataTables/DT_Quest.DT_Quest" ID%20Quest)
    (:then
      (Utilities|Map|Add (Variables|Default|GetQuests) ID%20Quest _returnvalue)
      (bind _keys (Utilities|Map|Keys (.Objetives (Utilities|Struct|BreakS_Quest _returnvalue))))
      (bind _returnvalue_2 (Game|ConstructObjectfromClass "/Game/Blueprints/QuestProgressItem.QuestProgressItem_C"))
      (bind _output_get (LocalVariables|SetNewQuestProgressItem _returnvalue_2))
      (Variables|/Game/Blueprints/QuestProgressItem.QuestProgressItem_C|SetIDQuest _output_get ID%20Quest)
      (Utilities|Array|Clear (LocalVariables|GetEnemys))
      (for _array_element _keys
        (Utilities|Array|Add (LocalVariables|GetEnemys) (.ACTOR (Utilities|Struct|BreakS_QuestObjective _array_element))))
      (Utilities|Array|Add (Variables|Default|GetKillingQuests) (LocalVariables|GetNewQuestProgressItem)))))

(fn UpdateQuestProgress
  (params (ID%20Quest :type Name) (ID%20Quest%20Objetive :type Name))
  (bind _keys (Utilities|Map|Keys (.Objetives (Utilities|Struct|BreakS_Quest (.Value (Utilities|Map|Find (Variables|Default|GetQuests) ID%20Quest))))))
  (for _array_element _keys
    _))