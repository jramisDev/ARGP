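; Mana manager component that holds its owner's current and maximum mana, with getters for both.
; On BeginPlay it sets mana to its initial value and starts a looping timer on the regeneration interval.
; Spending and regeneration functions adjust mana, clamp it between zero and the maximum, and broadcast the new value through ManaChanged.
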(event EventBeginPlay
  (Variables|Mana|SetMana (Variables|Mana|GetManaInitial))
  (Utilities|Time|SetTimerbyEvent (EventDispatchers|CreateEvent :!event RegenerateMana) (Variables|Mana|GetTimeManaRegeneration) true))

(fn GetMana
  (return (Variables|Mana|GetMana)))

(fn GetManaMax
  (return (Variables|Mana|GetManaMax)))

(fn RemoveMana
  (params (ManaCost :type Float%20%28double-precision%29))
  (bind _output_get (Variables|Mana|SetMana (Math|Float|Clamp(Float) (- (Variables|Mana|GetMana) ManaCost) 0.0 (Variables|Mana|GetManaMax))))
  (Default|CallManaChanged _output_get))

(fn RegenerateMana
  (bind _output_get (Variables|Mana|SetMana (Math|Float|Clamp(Float) (+ (Variables|Mana|GetManaRegeneration) (Variables|Mana|GetMana)) 0.0 (Variables|Mana|GetManaMax))))
  (Default|CallManaChanged _output_get))