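; Health manager component that tracks an actor's health and signals its death.
; Health starts at the maximum on BeginPlay, and the AnyDamage event subtracts damage, clamped between zero and the maximum.
; At zero health it calls YouHaveDie with the Controller from the damage event, then destroys the component.
; Getter functions expose current and maximum health.
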(event Custom|AnyDamage
  (params (Damage :type Float%20%28double-precision%29) (DamageType :type Damage%20Type%20Object%20Reference) (Controller :type Controller%20Object%20Reference))
  (bind _output_get (Variables|Health|SetHealth (Math|Float|Clamp(Float) (- (Variables|Health|GetHealth) Damage) 0.0 (Variables|Health|GetHealthMax))))
  (if (<= _output_get 0.0)
    (Default|CallYouHaveDie Controller)
    (Components|DestroyComponent)))

(event EventBeginPlay
  (Variables|Health|SetHealth (Variables|Health|GetHealthMax)))

(fn GetHealth
  (return (Variables|Health|GetHealth)))

(fn GetHealthMax
  (return (Variables|Health|GetHealthMax)))