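; Base player hero Blueprint that extends parent character logic with HUD updates, XP leveling and skill point spending.
; Health, mana and skill-use changes push values, cooldowns and loads to the HUD through a cached PC_Game reference.
; LevelUp uses DT_Level thresholds and grants skill points, which learning spends and removal refunds through the skill manager.
; It also positions a crosshair widget by look-trace distance and includes save/load/delete keys and per-tick skill-load debug text.
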(event EventBeginPlay
  (|CallParentFunction)
  (Utilities|FlowControl|Delay 0.2)
  (CallFunction|RefreshUI))

(event EventTick
  (params (DeltaSeconds :type Float%20%28single-precision%29))
  (bind _bpc_skillmanager (Variables|Default|GetBPC_SkillManager))
  (bind _loadsskills (Variables|/Game/Blueprints/Components/BPC_SkillManager.BPC_SkillManager_C|GetLoadsSkills _bpc_skillmanager))
  (bind _keys (Utilities|Map|Keys _loadsskills))
  (for _array_element _keys
    (Development|PrintText (Utilities|Text|FormatText "{s} / {c}" _array_element (.Value (Utilities|Map|Find _loadsskills _array_element))) true true "(R=0.000000,G=0.660000,B=1.000000,A=1.000000)" DeltaSeconds)))

(event Input|KeyboardEvents|P
  (params (Key :type Key%20Structure :default "None"))
  (:Pressed
    (bind _returnvalue (SaveGame|DeleteGameinSlot (Default|GetSlotName (CallFunction|GetGIRef))))
    (Development|PrintString (Utilities|String|ToString(Boolean) _returnvalue))))

(event Input|KeyboardEvents|F9
  (params (Key :type Key%20Structure :default "None"))
  (:Pressed
    (Default|SaveGame (CallFunction|GetGIRef) self)))

(event Input|KeyboardEvents|F10
  (params (Key :type Key%20Structure :default "None"))
  (:Pressed
    (Default|LoadGame (CallFunction|GetGIRef) self)
    (Default|RefreshSelectedSkills (CallFunction|GetHUDRef))))

(event Game|Damage|EventAnyDamage
  (params (Damage :type Float%20%28single-precision%29) (DamageType :type Damage%20Type%20Object%20Reference) (InstigatedBy :type Controller%20Object%20Reference) (DamageCauser :type Actor%20Object%20Reference))
  (|CallParentFunction Damage DamageType InstigatedBy DamageCauser)
  (Default|RefreshHP (CallFunction|GetHUDRef) (Default|GetHealth (Variables|Default|GetBPC_HealthManager))))

(event ManaChanged(BPC_ManaManager)
  (params (Mana :type Float%20%28double-precision%29))
  (Default|RefreshSP (CallFunction|GetHUDRef) Mana))

(fn ConstructionScript
  (|CallParentFunction))

(fn LookatDirection
  (params (Direction%20to%20Look%20At :type Vector%20%28by%20ref%29 :default "0, 0, 0"))
  (bind (_outhit _returnvalue) (|CallParentFunction Direction%20to%20Look%20At))
  (if _returnvalue
    (Transformation|SetRelativeLocation (Variables|Default|GetWidget) (Math|Vector|MakeVector 0.0 (Math|Float|Clamp(Float) (.Distance (Collision|BreakHitResult _outhit)) 1e+01 (Variables|Default|GetCrosshairDistance)) 9e+01) false false)
    (return "" true)
    (else
      (Transformation|SetRelativeLocation (Variables|Default|GetWidget) (Math|Vector|MakeVector 0.0 (Variables|Default|GetCrosshairDistance) 9e+01) false false)
      (return "" false))))

(fn GetPCRef
  (Variables|General|GetAs%20PC%20Game
    (:then
      _)
    (:else
      (bind _aspc_game (Utilities|Casting|CastToPC_Game (Pawn|GetController)))
      (Variables|General|SetAs%20PC%20Game _aspc_game)))
  (return (Variables|General|GetAs%20PC%20Game)))

(fn GetHUDRef
  (return (Default|GetHUDRef (CallFunction|GetPCRef))))

(fn UseSkillSlot
  (params (SkillToUse :type E_Actions%20Enum :default "NewEnumerator4"))
  (bind _bpc_skillmanager (Variables|Default|GetBPC_SkillManager))
  (bind (_loads _max_loads) (Default|GetLoadsSkills _bpc_skillmanager SkillToUse))
  (bind _skillused (|CallParentFunction SkillToUse))
  (if _skillused
    (Default|SetColdownforSkill (CallFunction|GetHUDRef) SkillToUse (Default|GetColdownforSlot (Variables|Default|GetBPC_SkillManager) SkillToUse))
    (Default|RefreshLoadsSkill (CallFunction|GetHUDRef) SkillToUse _loads _max_loads)
    (return _skillused)))

(fn RefreshUI
  (Default|RefreshSelectedSkills (CallFunction|GetHUDRef))
  (Default|RefreshHP (CallFunction|GetHUDRef) (Default|GetHealth (Variables|Default|GetBPC_HealthManager)))
  (Default|RefreshMaxHP (CallFunction|GetHUDRef) (Default|GetHealthMax (Variables|Default|GetBPC_HealthManager)))
  (Default|RefreshSP (CallFunction|GetHUDRef) (Default|GetMana (Variables|Default|GetBPC_ManaManager)))
  (Default|RefreshSPMax (CallFunction|GetHUDRef) (Default|GetManaMax (Variables|Default|GetBPC_ManaManager))))

(fn GainXP
  (params (XP :type Integer))
  (bind _output_get (Variables|Stats/Experience|SetXP (+ (Variables|Stats/Experience|GetXP) XP)))
  (if (>= _output_get (CallFunction|GetMaxXP))
    (CallFunction|LevelUp))
  (Default|UpdateXP (CallFunction|GetHUDRef) (Math|Conversions|ToFloat(Integer) (Variables|Stats/Experience|GetXP)) (Math|Conversions|ToFloat(Integer) (CallFunction|GetMaxXP))))

(fn GetMaxXP
  (bind _returnvalue (Utilities|GetDataTableRow "/Game/Blueprints/DataTables/DT_Level.DT_Level" (Utilities|String|StringToName (Utilities|String|ToString(Integer) (Variables|Stats/Experience|GetLevel))))
    (:then
      (return (.ExperienceMax (Utilities|Struct|BreakS_Level _returnvalue))))))

(fn LevelUp
  (Variables|Stats/Experience|SetXP (- (Variables|Stats/Experience|GetXP) (CallFunction|GetMaxXP)))
  (Math|Integer|IncrementInt (Variables|Stats/Experience|GetLevel)
    (:%20%20
      (Math|Integer|IncrementInt (Variables|Stats/Experience|GetSkillPoints)
        (:%20%20
          (Default|LevelUp (CallFunction|GetPCRef)))))))

(fn DoIHaveThisSkill
  (params (ItemToFind :type Name%20%28by%20ref%29))
  (return (Utilities|Array|ContainsItem (Variables|/Game/Blueprints/Components/BPC_SkillManager.BPC_SkillManager_C|GetAllAvailableSkills (Variables|Default|GetBPC_SkillManager)) ItemToFind)))

(fn LearnSkill
  (params (ID%20Skill :type Name%20%28by%20ref%29))
  (if (> (Variables|Stats/Experience|GetSkillPoints) 0)
    (bind _skill_learned (Default|LearnNewSkill (Variables|Default|GetBPC_SkillManager) ID%20Skill))
    (if _skill_learned
      (Math|Integer|DecrementInt (Variables|Stats/Experience|GetSkillPoints)))))

(fn RemoveSkill
  (params (ID%20Skill :type Name))
  (bind _skillremoved (Default|RemoveSkillLearned (Variables|Default|GetBPC_SkillManager) ID%20Skill))
  (if _skillremoved
    (Math|Integer|IncrementInt (Variables|Stats/Experience|GetSkillPoints))))