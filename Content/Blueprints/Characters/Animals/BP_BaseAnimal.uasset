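; Base animal character that wanders at random and can be tamed to follow a hero character.
; From BeginPlay it loops AI moves to random reachable points, pausing briefly after each successful arrival.
; Tame starts following on first use, then toggles between following and standing by.
; Both movement loops are self-calling events that repeat only on move success, with no retry on failure.
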(event Custom|FollowingHero
  (params (BaseCharacter :type BP%20Base%20Character%20Object%20Reference))
  (if (Variables|Animal|GetIsFollowing)
    (AI|AIMoveTo self "0, 0, 0" BaseCharacter 2e+02 false
      (:OnSuccess
        (Utilities|FlowControl|Delay 1.0)
        (CallFunction|FollowingHero BaseCharacter)))))

(event Custom|StandBy
  (Components|Movement|StopMovementImmediately (Variables|Character|GetCharacterMovement)))

(event Custom|RandomMovement
  (AI|AIMoveTo self (.RandomLocation (AI|Navigation|GetRandomReachablePointinRadius (Transformation|GetActorLocation) 2e+03 0 0)) 0 5.0 false
    (:OnSuccess
      (Utilities|FlowControl|Delay (Math|Random|RandomFloatinRange 1.0 5.0))
      (CallFunction|RandomMovement))))

(event EventBeginPlay
  (CallFunction|RandomMovement))

(event EventTame
  (params (BaseCharacter :type BP%20Base%20Character%20Object%20Reference))
  (if (Variables|Animal|GetIsTamed)
    (if (Variables|Animal|GetIsFollowing)
      (Variables|Animal|SetIsFollowing false)
      (CallFunction|Standby)
      (else
        (Variables|Animal|SetIsFollowing true)
        (CallFunction|FollowingHero BaseCharacter)))
    (else
      (Variables|Animal|SetIsTamed true)
      (Variables|Animal|SetIsFollowing true)
      (CallFunction|FollowingHero BaseCharacter))))

(fn ConstructionScript
  (|CallParentFunction))