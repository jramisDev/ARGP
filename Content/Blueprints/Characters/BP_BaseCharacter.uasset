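; Base character that moves and aims on the ground plane from 2D input vectors, with jumping, skills, damage and death.
; Aiming yaws only the mesh toward a crosshair point and line-traces to it; skills spawn through the skill manager component along that facing.
; Damage reaches the health manager component unless dodging; death grants the killer's hero XP and destroys the actor.
; Player loading goes through a cached game instance, with the save slot named from the PlayerState.
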(event Custom|MoveInDirection
  (params (InVector2D :type Vector%202D%20Structure))
  (Pawn|Input|AddMovementInput (Math|Conversions|ToVector(Vector2D) InVector2D) 1.0 false))

(event Custom|RotateDirection
  (params (InVector2D :type Vector%202D%20Structure))
  (bind _returnvalue (Math|Conversions|ToVector(Vector2D) InVector2D))
  (bind _returnvalue_2 (Transformation|GetActorLocation))
  (bind _crosshairdistance (Variables|Movement|GetCrosshairDistance))
  (bind _returnvalue_3 (* _returnvalue _crosshairdistance))
  (bind _returnvalue_4 (+ _returnvalue_2 _returnvalue_3))
  (Rendering|Debug|DrawDebugArrow _returnvalue_2 _returnvalue_4 5.0 "(R=0.000000,G=1.000000,B=0.923001,A=1.000000)" 0.0 2.0)
  (CallFunction|LookatDirection _returnvalue_4))

(event Custom|StartJump
  (Variables|Movement|SetIsJumping true)
  (Character|Jump))

(event Custom|StopJump
  (Character|StopJumping))

(event EventOnLanded
  (params (Hit :type Hit%20Result%20Structure%20%28by%20ref%29)))

(event Custom|StopUsingSkill
  (Default|StopUseSkill (Variables|Default|GetBPC_SkillManager)))

(event YouHaveDie(BPC_HealthManager)
  (params (Controller :type Controller%20Object%20Reference))
  (bind _aspc_game (Utilities|Casting|CastToPC_Game Controller)
    (:then
      (Default|GainXP (Default|GetHeroRef _aspc_game) (Variables|Stats/Experience|GetIncreaseXPOnKill)))
    (:CastFailed
      _))
  (CallFunction|StartDying))

(event Custom|StartDying
  (Actor|DestroyActor))

(event Game|Damage|EventAnyDamage
  (params (Damage :type Float%20%28single-precision%29) (DamageType :type Damage%20Type%20Object%20Reference) (InstigatedBy :type Controller%20Object%20Reference) (DamageCauser :type Actor%20Object%20Reference))
  (if (not (Variables|Movement|GetIsDodgin))
    (Default|AnyDamage (Variables|Default|GetBPC_HealthManager) Damage DamageType InstigatedBy)))

(fn ConstructionScript)

(fn LookatDirection
  (params (Direction%20to%20Look%20At :type Vector%20%28by%20ref%29))
  (Transformation|SetWorldRotation (Variables|Character|GetMesh) (Math|Rotator|MakeRotator 0.0 0.0 (- (.yaw (Math|Rotator|FindLookatRotation (Transformation|GetActorLocation) Direction%20to%20Look%20At)) 9e+01)) false false)
  (bind (_outhit _returnvalue) (Collision|LineTraceByChannel (Transformation|GetActorLocation) Direction%20to%20Look%20At "TraceTypeQuery1" false 0 "None" true "(R=1.000000,G=0.000000,B=0.000000,A=1.000000)" "(R=0.000000,G=1.000000,B=0.000000,A=1.000000)" 0.1))
  (return _outhit _returnvalue))

(fn UseSkillSlot
  (params (SkillToUse :type E_Actions%20Enum :default "NewEnumerator4"))
  (bind _mesh (Variables|Character|GetMesh))
  (bind _returnvalue (Transformation|GetWorldRotation _mesh))
  (bind _usedskill (Default|TrytoUseSkill (Variables|Default|GetBPC_SkillManager) (Transformation|GetWorldLocation (Variables|Default|GetSkillSpawn)) (Math|Rotator|MakeRotator (.roll _returnvalue) (.pitch _returnvalue) (+ (.yaw _returnvalue) 9e+01)) SkillToUse))
  (return _usedskill))

(fn GetGIRef
  (Variables|General|GetAs%20GI%202DGame
    (:then
      _)
    (:else
      (bind _asgi_game (Utilities|Casting|CastToGI_Game (Game|GetGameInstance)))
      (Variables|General|SetAs%20GI%202DGame _asgi_game)))
  (return (Variables|General|GetAs%20GI%202DGame)))

(fn LoadPlayer
  (Default|SetSlotName (CallFunction|GetGIRef) (Utilities|GetDisplayName (Variables|/Script/Engine.Controller|GetPlayerState (Pawn|GetController))))
  (Default|LoadGame (CallFunction|GetGIRef) self))