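; GM_Game is the game mode that provides access to the player's SG_SaveGame object.
; LoadGame reads it from a single fixed slot, or creates a new instance when no save exists, and caches it in SGSaveGame.
; Despite its name, SaveGame only returns that cached object, loading it first if invalid; nothing writes to disk.
; BeginPlay is empty, and a second-player CreatePlayer call is left unconnected.
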(event EventBeginPlay)

(fn ConstructionScript)

(fn LoadGame
  (params (SaveGame :type SG%20Save%20Game%20Object%20Reference))
  (bind _returnvalue (SaveGame|DoesSaveGameExist (SaveGame|GetSaveGameSlotName)))
  (if _returnvalue
    (bind _returnvalue_2 (SaveGame|LoadGamefromSlot (SaveGame|GetSaveGameSlotName)))
    (bind _assg_save_game (Utilities|Casting|CastToSG_SaveGame _returnvalue_2))
    (Variables|SaveGame|SetSG_SaveGame _assg_save_game)
    (else
      (bind _returnvalue_3 (SaveGame|CreateSaveGameObject "/Game/Blueprints/SaveGame/SG_SaveGame.SG_SaveGame_C"))
      (Variables|SaveGame|SetSG_SaveGame _returnvalue_3)))
  (return (Variables|SaveGame|GetSG_SaveGame)))

(fn SaveGame
  (Variables|SaveGame|GetSG_SaveGame
    (:then
      _)
    (:else
      (SaveGame|LoadGame)))
  (return (Variables|SaveGame|GetSG_SaveGame)))

(fn GetSaveGameSlotName
  (return (Utilities|String|Append "SaveGamePlayer" "")))