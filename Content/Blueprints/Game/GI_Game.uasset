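; GI_Game, apparently the game instance, holds the player's SG_SaveGame object and a save slot name built from a controlled name plus "PlayerData".
; GetPlayerData returns that object, calling LoadGame first if it is invalid.
; LoadGame and SaveGame have empty bodies: their logic to load or create the slot's save and write character data is disconnected and never runs.
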(fn GetPlayerData
  (params (BaseCharacter :type BP%20Base%20Character%20Object%20Reference))
  (Variables|Default|GetSG_game
    (:then
      _)
    (:else
      (CallFunction|LoadGame BaseCharacter)))
  (return (Variables|Default|GetSG_game)))

(fn SetSlotName
  (params (ControlledName :type String))
  (Variables|Default|SetSlotName (Utilities|String|Append ControlledName "PlayerData")))

(fn GetSlotName
  (return (Variables|Default|GetSlotName)))

(fn LoadGame
  (params (Base%20Character :type BP%20Base%20Character%20Object%20Reference)))

(fn SaveGame
  (params (Base%20Character :type BP%20Base%20Character%20Object%20Reference)))