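; PC_Game is the gameplay player controller, routing Enhanced Input to the controlled BP_BaseCharacter for movement, jumping and four skill slots.
; Pause and skill tree inputs toggle UI mode, swapping IMC_Game and IMC_UI, while HUD_Game handles menus, navigation and level-up notices.
; Outside UI mode, a per-tick cursor trace aims the character until rotate input disables mouse aiming.
; Lazy getters cache character, hero, HUD and game instance references.
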(event EventBeginPlay
  (Utilities|FlowControl|Delay 0.2)
  (Input|AddMappingContext (PlayerController|LocalPlayerSubsystems|GetEnhancedInputLocalPlayerSubsystem) "/Game/Input/Game/IMC_Game.IMC_Game" 0 "(bIgnoreAllPressedKeysUntilRelease=True,bForceImmediately=False,bNotifyUserSettings=False)")
  (Class|WidgetBlueprintLibrary|SetFocustoGameViewport)
  (Variables|Default|SetIsMouse (== (Game|GetPlayerController 0) self)))

(event EventTick
  (params (DeltaSeconds :type Float%20%28single-precision%29))
  (if (and (Variables|Default|GetIsMouse) (not (Variables|Default|GetisUIMode)))
    (CallFunction|RotatePlayer)))

(event Input|EnhancedActionEvents|EnhancedInputActionIA_SkillTree
  (params (ActionValue :type Boolean) (ElapsedSeconds :type Float%20%28double-precision%29) (TriggeredSeconds :type Float%20%28double-precision%29) (InputAction :type Input%20Action%20Object%20Reference :default "/Game/Input/Game/IA_SkillTree.IA_SkillTree"))
  (:Started
    (CallFunction|ToggleUIMode (not (Variables|Default|GetisUIMode)))
    (Default|ToggleSkillTree (CallFunction|GetHUDRef))))

(event Input|EnhancedActionEvents|EnhancedInputActionIA_Cancel
  (params (ActionValue :type Boolean) (ElapsedSeconds :type Float%20%28double-precision%29) (TriggeredSeconds :type Float%20%28double-precision%29) (InputAction :type Input%20Action%20Object%20Reference :default "/Game/Input/UI/IA_Cancel.IA_Cancel"))
  (:Started
    (Default|ConfirmCancel (CallFunction|GetHUDRef) true)))

(event Input|EnhancedActionEvents|EnhancedInputActionIA_Pause
  (params (ActionValue :type Boolean) (ElapsedSeconds :type Float%20%28double-precision%29) (TriggeredSeconds :type Float%20%28double-precision%29) (InputAction :type Input%20Action%20Object%20Reference :default "/Game/Input/Game/IA_Pause.IA_Pause"))
  (:Started
    (CallFunction|ToggleUIMode (not (Variables|Default|GetisUIMode)))
    (Default|ToggleSkillBook (CallFunction|GetHUDRef))
    (Default|LoadPlayer (.AsBP%20Base%20Character (Utilities|Casting|CastToBP_BaseCharacter (Pawn|GetControlledPawn))))
    (Default|RefreshSelectedSkills (CallFunction|GetHUDRef))))

(event Input|EnhancedActionEvents|EnhancedInputActionIA_MoveUI
  (params (ActionValue :type Vector%202D%20Structure) (ElapsedSeconds :type Float%20%28double-precision%29) (TriggeredSeconds :type Float%20%28double-precision%29) (InputAction :type Input%20Action%20Object%20Reference :default "/Game/Input/UI/IA_MoveUI.IA_MoveUI"))
  (:Started
    (Default|InputMove (CallFunction|GetHUDRef) ActionValue)))

(event Input|EnhancedActionEvents|EnhancedInputActionIA_Confirm
  (params (ActionValue :type Boolean) (ElapsedSeconds :type Float%20%28double-precision%29) (TriggeredSeconds :type Float%20%28double-precision%29) (InputAction :type Input%20Action%20Object%20Reference :default "/Game/Input/UI/IA_Confirm.IA_Confirm"))
  (:Started
    (Default|ConfirmCancel (CallFunction|GetHUDRef) true)))

(event Input|EnhancedActionEvents|EnhancedInputActionIA_Move
  (params (ActionValue :type Vector%202D%20Structure) (ElapsedSeconds :type Float%20%28double-precision%29) (TriggeredSeconds :type Float%20%28double-precision%29) (InputAction :type Input%20Action%20Object%20Reference :default "/Game/Input/Game/IA_Move.IA_Move"))
  (Default|MoveinDirection (CallFunction|GetBaseCharacterRef) ActionValue))

(event Input|EnhancedActionEvents|EnhancedInputActionIA_Jump
  (params (ActionValue :type Boolean) (ElapsedSeconds :type Float%20%28double-precision%29) (TriggeredSeconds :type Float%20%28double-precision%29) (InputAction :type Input%20Action%20Object%20Reference :default "/Game/Input/Game/IA_Jump.IA_Jump"))
  (bind _as_bp_base_character (CallFunction|GetBaseCharacterRef))
  (:Started
    (Default|StartJump _as_bp_base_character))
  (:Completed
    (Default|StopJump _as_bp_base_character)))

(event Input|EnhancedActionEvents|EnhancedInputActionIA_Rotate
  (params (ActionValue :type Vector%202D%20Structure) (ElapsedSeconds :type Float%20%28double-precision%29) (TriggeredSeconds :type Float%20%28double-precision%29) (InputAction :type Input%20Action%20Object%20Reference :default "/Game/Input/Game/IA_Rotate.IA_Rotate"))
  (Default|RotateDirection (CallFunction|GetBaseCharacterRef) ActionValue))

(event Input|EnhancedActionEvents|EnhancedInputActionIA_Rotate
  (params (ActionValue :type Vector%202D%20Structure) (ElapsedSeconds :type Float%20%28double-precision%29) (TriggeredSeconds :type Float%20%28double-precision%29) (InputAction :type Input%20Action%20Object%20Reference :default "/Game/Input/Game/IA_Rotate.IA_Rotate"))
  (Utilities|FlowControl|DoOnce false
    (:Completed
      (Variables|Default|SetIsMouse false))))

(event Input|EnhancedActionEvents|EnhancedInputActionIA_ThirdSkill
  (params (ActionValue :type Boolean) (ElapsedSeconds :type Float%20%28double-precision%29) (TriggeredSeconds :type Float%20%28double-precision%29) (InputAction :type Input%20Action%20Object%20Reference :default "/Game/Input/Game/IA_ThirdSkill.IA_ThirdSkill"))
  (bind _as_bp_base_character (CallFunction|GetBaseCharacterRef))
  (:Triggered
    (Default|UseSkillSlot _as_bp_base_character "NewEnumerator2"))
  (:Completed
    (Default|StopUsingSkill _as_bp_base_character)))

(event Input|EnhancedActionEvents|EnhancedInputActionIA_UltimateSkill
  (params (ActionValue :type Boolean) (ElapsedSeconds :type Float%20%28double-precision%29) (TriggeredSeconds :type Float%20%28double-precision%29) (InputAction :type Input%20Action%20Object%20Reference :default "/Game/Input/Game/IA_UltimateSkill.IA_UltimateSkill"))
  (bind _as_bp_base_character (CallFunction|GetBaseCharacterRef))
  (:Triggered
    (Default|UseSkillSlot _as_bp_base_character "NewEnumerator3"))
  (:Completed
    (Default|StopUsingSkill _as_bp_base_character)))

(event Input|EnhancedActionEvents|EnhancedInputActionIA_PrimarySkill
  (params (ActionValue :type Boolean) (ElapsedSeconds :type Float%20%28double-precision%29) (TriggeredSeconds :type Float%20%28double-precision%29) (InputAction :type Input%20Action%20Object%20Reference :default "/Game/Input/Game/IA_PrimarySkill.IA_PrimarySkill"))
  (bind _as_bp_base_character (CallFunction|GetBaseCharacterRef))
  (:Triggered
    (Default|UseSkillSlot _as_bp_base_character "NewEnumerator0"))
  (:Completed
    (Default|StopUsingSkill _as_bp_base_character)))

(event Input|EnhancedActionEvents|EnhancedInputActionIA_SecondarySkill
  (params (ActionValue :type Boolean) (ElapsedSeconds :type Float%20%28double-precision%29) (TriggeredSeconds :type Float%20%28double-precision%29) (InputAction :type Input%20Action%20Object%20Reference :default "/Game/Input/Game/IA_SecondarySkill.IA_SecondarySkill"))
  (bind _as_bp_base_character (CallFunction|GetBaseCharacterRef))
  (:Triggered
    (Default|UseSkillSlot _as_bp_base_character "NewEnumerator1"))
  (:Completed
    (Default|StopUsingSkill _as_bp_base_character)))

(fn ConstructionScript)

(fn GetBaseCharacterRef
  (Variables|Default|GetAs%20BP%20Base%20Character
    (:then
      _)
    (:else
      (bind _asbp_base_character (Utilities|Casting|CastToBP_BaseCharacter (Pawn|GetControlledPawn)))
      (Variables|Default|SetAs%20BP%20Base%20Character _asbp_base_character)))
  (return (Variables|Default|GetAs%20BP%20Base%20Character)))

(fn ToggleUIMode
  (params (UI%20Mode :type Boolean))
  (bind _self self)
  (bind _returnvalue (PlayerController|LocalPlayerSubsystems|GetEnhancedInputLocalPlayerSubsystem _self))
  (if UI%20Mode
    (Variables|Default|SetisUIMode true)
    (Input|SetInputModeGameandUI self 0 "DoNotLock" true false)
    (Variables|Default|SetbShowMouseCursor true)
    (Input|AddMappingContext _returnvalue "/Game/Input/UI/IMC_UI.IMC_UI" 0 "(bIgnoreAllPressedKeysUntilRelease=True,bForceImmediately=False,bNotifyUserSettings=False)")
    (Input|RemoveMappingContext _returnvalue "/Game/Input/Game/IMC_Game.IMC_Game" "(bIgnoreAllPressedKeysUntilRelease=True,bForceImmediately=False,bNotifyUserSettings=False)")
    (else
      (Variables|Default|SetisUIMode false)
      (Input|SetInputModeGameOnly self false)
      (Variables|Default|SetbShowMouseCursor false)
      (Input|AddMappingContext _returnvalue "/Game/Input/Game/IMC_Game.IMC_Game" 0 "(bIgnoreAllPressedKeysUntilRelease=True,bForceImmediately=False,bNotifyUserSettings=False)")
      (Input|RemoveMappingContext _returnvalue "/Game/Input/UI/IMC_UI.IMC_UI" "(bIgnoreAllPressedKeysUntilRelease=True,bForceImmediately=False,bNotifyUserSettings=False)"))))

(fn GetHUDRef
  (Variables|Default|GetAs%20HUD%20Game
    (:then
      _)
    (:else
      (bind _ashud_game (Utilities|Casting|CastToHUD_Game (HUD|GetHUD)))
      (Variables|Default|SetAs%20HUD%20Game _ashud_game)))
  (return (Variables|Default|GetAs%20HUD%20Game)))

(fn RotatePlayer
  (bind (_worldlocation _worlddirection) (Game|Player|ConvertMouseLocationToWorldSpace))
  (bind (_outhit _returnvalue) (Collision|LineTraceByChannel _worldlocation (+ _worldlocation (* _worlddirection 1.5e+04)) "TraceTypeQuery1" false 0 "None"))
  (if _returnvalue
    (Default|LookatDirection (CallFunction|GetBaseCharacterRef) (.Location (Collision|BreakHitResult _outhit)))))

(fn GetGIRef
  (Variables|Default|GetAs%20GI%202DGame
    (:then
      _)
    (:else
      (bind _asgi_game (Utilities|Casting|CastToGI_Game (Game|GetGameInstance)))
      (Variables|Default|SetAs%20GI%202DGame _asgi_game)))
  (return (Variables|Default|GetAs%20GI%202DGame)))

(fn GetHeroRef
  (Variables|Default|GetAs%20BP%20Base%20Hero
    (:then
      _)
    (:else
      (bind _asbp_base_hero (Utilities|Casting|CastToBP_BaseHero (Pawn|GetControlledPawn)))
      (Variables|Default|SetAs%20BP%20Base%20Hero _asbp_base_hero)))
  (return (Variables|Default|GetAs%20BP%20Base%20Hero)))

(fn LevelUp
  (Default|NotifyLevelUp (CallFunction|GetHUDRef)))